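; BP_Key_Green is the green variant of a key object, with its visual tint applied at construction time.
; After calling the parent construction script, it creates dynamic material instances on Frame1 and Frame2 from M_Frame1 and M_Frame2, setting each "Base Color" parameter to the same green.
; The event graph holds only disabled placeholder events, so this Blueprint's graphs add no gameplay logic of their own.
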(event EventBeginPlay
  (|CallParentFunction) ; This node is disabled and will not be called.\nDrag off pins to build functionality.
)

(event Collision|EventActorBeginOverlap
  (params (OtherActor :type Actor%20Object%20Reference))
  (|CallParentFunction OtherActor) ; This node is disabled and will not be called.\nDrag off pins to build functionality.
)

(event EventTick
  (params (DeltaSeconds :type Float%20%28single-precision%29))
  (|CallParentFunction DeltaSeconds) ; This node is disabled and will not be called.\nDrag off pins to build functionality.
)

(fn ConstructionScript
  (|CallParentFunction)
  (bind _returnvalue (Rendering|Material|CreateDynamicMaterialInstance (Variables|Default|GetFrame1) 0 "/Game/Objects/Key/M_Frame1.M_Frame1" "None" :!class /Script/Engine.PrimitiveComponent))
  (Rendering|Material|SetVectorParameterValue _returnvalue "Base Color" "(R=0.084174,G=0.774306,B=0.026886,A=1.000000)" :!class /Script/Engine.MaterialInstanceDynamic)
  (bind _returnvalue_2 (Rendering|Material|CreateDynamicMaterialInstance (Variables|Default|GetFrame2) 0 "/Game/Objects/Key/M_Frame2.M_Frame2" "None" :!class /Script/Engine.PrimitiveComponent))
  (Rendering|Material|SetVectorParameterValue _returnvalue_2 "Base Color" "(R=0.084174,G=0.774306,B=0.026886,A=1.000000)" :!class /Script/Engine.MaterialInstanceDynamic))