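; Interactable totem of a green, blue or red type that activates when the GameMode reports the matching key picked up.
; Activation starts the square's timeline, raises the totem's emissive and has the GameMode count active totems and check for completion.
; Interact also spawns a BP_KeyFix regardless of that check, coloring its two frames by type through dynamic materials.
; The construction script creates the totem's own dynamic material from its base color and emissive.
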(event Custom|ActiveGreenTotem
  (bind _game_mode_refer (Variables|Default|GetGame%20Mode%20Refer))
  ;[1 1 1] Active Totems - isPickKey - PlayTotemAnimation
  (if (Variables|/Game/GameLogic/BP_Gameplay_GameMode.BP_Gameplay_GameMode_C|GetIsPickUpKeyGreen (Variables|Default|GetGame%20Mode%20Refer))
    (Components|Timeline|PlayfromStart (Variables|Default|GetSquareTimeline))
    (Rendering|Material|SetScalarParameterValue (Variables|Default|GetTotemMaterial) "Emissive" (Variables|Default|GetEmissiveIntensityActive) :!class /Script/Engine.MaterialInstanceDynamic)
    (Default|IncrementNumberTotemsActive _game_mode_refer)
    (Default|CheckAllTotemsActive _game_mode_refer)))

(event Custom|ActiveBlueTotem
  (bind _game_mode_refer (Variables|Default|GetGame%20Mode%20Refer))
  ;[1 1 1] Active Totems - isPickKey - PlayTotemAnimation
  (if (Variables|/Game/GameLogic/BP_Gameplay_GameMode.BP_Gameplay_GameMode_C|GetIsPickUpKeyBlue (Variables|Default|GetGame%20Mode%20Refer))
    (Components|Timeline|PlayfromStart (Variables|Default|GetSquareTimeline))
    (Rendering|Material|SetScalarParameterValue (Variables|Default|GetTotemMaterial) "Emissive" (Variables|Default|GetEmissiveIntensityActive) :!class /Script/Engine.MaterialInstanceDynamic)
    (Default|IncrementNumberTotemsActive _game_mode_refer)
    (Default|CheckAllTotemsActive _game_mode_refer)))

(event Custom|ActiveRedTotem
  (bind _game_mode_refer (Variables|Default|GetGame%20Mode%20Refer))
  ;[1 1 1] Active Totems - isPickKey - PlayTotemAnimation
  (if (Variables|/Game/GameLogic/BP_Gameplay_GameMode.BP_Gameplay_GameMode_C|GetIsPickUpKeyRed (Variables|Default|GetGame%20Mode%20Refer))
    (Components|Timeline|PlayfromStart (Variables|Default|GetSquareTimeline))
    (Rendering|Material|SetScalarParameterValue (Variables|Default|GetTotemMaterial) "Emissive" (Variables|Default|GetEmissiveIntensityActive) :!class /Script/Engine.MaterialInstanceDynamic)
    (Default|IncrementNumberTotemsActive _game_mode_refer)
    (Default|CheckAllTotemsActive _game_mode_refer)))

(event EventInteract
  ;[1 1 1] Blueprint Interfase Interact - Active Totem - Spawn Key - Create Material
  (switch Utilities|FlowControl|Switch|SwitchonEKeys (Variables|Default|GetTotemType)
    (:NewEnumerator0
      (CallFunction|ActiveGreenTotem)
      (bind _returnvalue (CallFunction|SpawnKey))
      (CallFunction|CreateKeyMaterial (Variables|/Game/Objects/Key/BP_KeyFix.BP_KeyFix_C|GetFrame1 _returnvalue) (Variables|/Game/Objects/Key/BP_KeyFix.BP_KeyFix_C|GetFrame2 _returnvalue) "(R=0.082353,G=0.776471,B=0.023529,A=1.000000)"))
    (:NewEnumerator1
      (CallFunction|ActiveBlueTotem)
      (bind _returnvalue_2 (CallFunction|SpawnKey))
      (CallFunction|CreateKeyMaterial (Variables|/Game/Objects/Key/BP_KeyFix.BP_KeyFix_C|GetFrame1 _returnvalue_2) (Variables|/Game/Objects/Key/BP_KeyFix.BP_KeyFix_C|GetFrame2 _returnvalue_2) "(R=0.000000,G=0.019608,B=1.000000,A=1.000000)"))
    (:NewEnumerator2
      (CallFunction|ActiveRedTotem)
      (bind _returnvalue_3 (CallFunction|SpawnKey))
      (CallFunction|CreateKeyMaterial (Variables|/Game/Objects/Key/BP_KeyFix.BP_KeyFix_C|GetFrame1 _returnvalue_3) (Variables|/Game/Objects/Key/BP_KeyFix.BP_KeyFix_C|GetFrame2 _returnvalue_3) "(R=1.000000,G=0.000000,B=0.003922,A=1.000000)"))))

(event EventBeginPlay
  (bind _asbp_gameplay_game_mode (Utilities|Casting|CastToBP_Gameplay_GameMode (Game|GetGameMode)))
  (Variables|Default|SetGame%20Mode%20Refer _asbp_gameplay_game_mode))

(fn ConstructionScript
  (bind _returnvalue (Rendering|Material|CreateDynamicMaterialInstance (Variables|Default|GetTotemBase) 1 "/Game/Objects/Totem/02_-_Default.02_-_Default" "None" :!class /Script/Engine.PrimitiveComponent))
  (bind _output_get (Variables|Default|SetTotemMaterial _returnvalue))
  (Rendering|Material|SetScalarParameterValue _output_get "Emissive" (Variables|Default|GetEmissiveIntensity) :!class /Script/Engine.MaterialInstanceDynamic)
  (Rendering|Material|SetVectorParameterValue _output_get "Param" (Variables|Default|GetBaseColor) :!class /Script/Engine.MaterialInstanceDynamic))

(fn SpawnKey
  (bind _returnvalue (Game|SpawnActorfromClass "/Game/Objects/Key/BP_KeyFix.BP_KeyFix_C" (Transformation|GetWorldTransform (Variables|Default|GetKeySpawnTrans)) "Undefined" 0 0))
  (return _returnvalue))

(fn CreateKeyMaterial
  (params (Target :type Primitive%20Component%20Object%20Reference) (Target2 :type Primitive%20Component%20Object%20Reference) (Color :type Linear%20Color%20Structure))
  (bind _returnvalue (Rendering|Material|CreateDynamicMaterialInstance Target 0 "/Game/Objects/Totem/02_-_Default.02_-_Default" "None" :!class /Script/Engine.PrimitiveComponent))
  (Rendering|Material|SetVectorParameterValue _returnvalue "Param" Color :!class /Script/Engine.MaterialInstanceDynamic)
  (Rendering|Material|SetScalarParameterValue _returnvalue "Emissive" 0.0 :!class /Script/Engine.MaterialInstanceDynamic)
  (bind _returnvalue_2 (Rendering|Material|CreateDynamicMaterialInstance Target2 0 "/Game/Objects/Totem/02_-_Default.02_-_Default" "None" :!class /Script/Engine.PrimitiveComponent))
  (Rendering|Material|SetVectorParameterValue _returnvalue_2 "Param" Color :!class /Script/Engine.MaterialInstanceDynamic)
  (Rendering|Material|SetScalarParameterValue _returnvalue_2 "Emissive" 8.0 :!class /Script/Engine.MaterialInstanceDynamic))