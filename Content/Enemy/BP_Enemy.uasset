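; BP_Enemy is a stationary shooter enemy that turns toward the player and fires projectiles on a looping timer once the player overlaps its capsule or hits it.
; A DoOnce gates the timer, with events to stop, reset and restart aggression.
; Hits reduce health, briefly change a sphere material parameter, and destroy it at zero.
; BeginPlay randomizes a vertical bobbing timeline's height and rate, though no wire starts that timeline.
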(event OnComponentBeginOverlap(Capsule)
  (params (OverlappedComponent :type Primitive%20Component%20Object%20Reference) (OtherActor :type Actor%20Object%20Reference) (OtherComp :type Primitive%20Component%20Object%20Reference) (OtherBodyIndex :type Integer) (bFromSweep :type Boolean) (SweepResult :type Hit%20Result%20Structure%20%28by%20ref%29))
  ;[1 1 1] Overlap - Set HeroOnSight
  (Variables|Default|SetIsHeroOnSight true))

(event OnComponentEndOverlap(Capsule)
  (params (OverlappedComponent :type Primitive%20Component%20Object%20Reference) (OtherActor :type Actor%20Object%20Reference) (OtherComp :type Primitive%20Component%20Object%20Reference) (OtherBodyIndex :type Integer))
  ;[1 1 1] Overlap - Set HeroOnSight
)

(event Custom|StopEnemy
  ;[1 1 1] Stop Enemy
  (Utilities|Time|ClearTimerbyFunctionName 0 "Fire"))

(event Custom|RestartEnemyFire
  ;[1 1 1] Set Actor Rot
  (Utilities|FlowControl|DoOnce false) ; enters at Reset
)

(event Custom|RestartEnemy
  ;[1 1 1] Restart Enemy
  (Variables|Default|SetIsHeroOnSight false)
  (Variables|Default|SetIsHeroHere false))

(event Custom|EventDead)

(event EventBeginPlay
  (bind _returnvalue (Transformation|GetActorLocation))
  (Utilities|FlowControl|Sequence
    (:then_0
      ;[1 1 1] Set Start End Location/Set Play Rate
      (Variables|Default|SetStartLocation _returnvalue)
      (Variables|Default|SetEndLocation (+ _returnvalue (Math|Vector|MakeVector 0.0 0.0 (Math|Random|RandomFloatinRange 5e+01 1e+02))))
      (Components|Timeline|SetPlayRate (Variables|Default|GetEnemyLoop) (Math|Random|RandomFloatinRange 1.0 2.0)))
    (:then_1
      ;[1 1 1] Cast to HeroChar
      (bind _asbp_haro_char (Utilities|Casting|CastToBP_HaroChar (Game|GetPlayerCharacter 0)))
      (Variables|Default|SetHaroCharRefer _asbp_haro_char))))

(event Collision|EventHit
  (params (MyComp :type Primitive%20Component%20Object%20Reference) (Other :type Actor%20Object%20Reference) (OtherComp :type Primitive%20Component%20Object%20Reference) (bSelfMoved :type Boolean) (HitLocation :type Vector :default "0, 0, 0") (HitNormal :type Vector :default "0, 0, 0") (NormalImpulse :type Vector :default "0, 0, 0") (Hit :type Hit%20Result%20Structure%20%28by%20ref%29))
  ;[1 1 1] Hit
  (Variables|Default|SetIsHeroHere true)
  (Variables|Default|SetEnemyHealth (- (Variables|Default|GetEnemyHealth) (Variables|Default|GetDamageTaken)))
  (if (<= (Variables|Default|GetEnemyHealth) 0.0)
    (CallFunction|EventDead)
    (Actor|DestroyActor)
    (else
      (Rendering|Material|SetScalarParameterValueonMaterials (Variables|Default|GetSphere) "None" 1.0)
      (Utilities|FlowControl|Delay 0.1)
      (Rendering|Material|SetScalarParameterValueonMaterials (Variables|Default|GetSphere) "None" 9e+01))))

(event EventTick
  (params (DeltaSeconds :type Float%20%28single-precision%29))
  ;[1 1 1] Set Actor Rot
  (if (or (Variables|Default|GetIsHeroOnSight) (Variables|Default|GetIsHeroHere))
    (Utilities|FlowControl|Sequence
      (:then_0
        (Transformation|SetActorRotation (Math|Rotator|FindLookatRotation (Transformation|GetActorLocation) (Transformation|GetActorLocation (Variables|Default|GetHaroCharRefer)))))
      (:then_1
        (Utilities|FlowControl|DoOnce false
          (:Completed
            (Utilities|Time|SetTimerbyFunctionName 0 "Fire" (/ 1.0 (Variables|Default|GetShoodPerSecond)) true)))))))

(fn ConstructionScript)

(fn Fire
  (Game|SpawnActorfromClass "/Game/Enemy/BP_ProjectilEnemy.BP_ProjectilEnemy_C" (Transformation|GetWorldTransform (Variables|Default|GetArrowProjectil)) "Undefined" 0 0))