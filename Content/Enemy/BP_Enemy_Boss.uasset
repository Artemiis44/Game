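; BP_Enemy_Boss is a boss enemy Blueprint that reports its death to the gameplay game mode.
; On BeginPlay it runs the parent logic, then casts and caches the BP_Gameplay_GameMode reference.
; Its EventDead event increments the game mode's NumberOfEnemyBossesDead counter and prints the new total for debugging.
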(event EventBeginPlay
  (|CallParentFunction)
  (bind _asbp_gameplay_game_mode (Utilities|Casting|CastToBP_Gameplay_GameMode (Game|GetGameMode)))
  (Variables|Default|SetGameplayGameModeRefer _asbp_gameplay_game_mode))

(event Collision|EventActorBeginOverlap
  (params (OtherActor :type Actor%20Object%20Reference)))

(event EventTick
  (params (DeltaSeconds :type Float%20%28single-precision%29))
  (|CallParentFunction DeltaSeconds) ; This node is disabled and will not be called.\nDrag off pins to build functionality.
)

(event EventEventDead
  (bind _gameplaygamemoderefer (Variables|Default|GetGameplayGameModeRefer))
  (bind _output_get (Variables|/Game/GameLogic/BP_Gameplay_GameMode.BP_Gameplay_GameMode_C|SetNumberOfEnemyBossesDead _gameplaygamemoderefer (+ (Variables|/Game/GameLogic/BP_Gameplay_GameMode.BP_Gameplay_GameMode_C|GetNumberOfEnemyBossesDead _gameplaygamemoderefer) 1)))
  (Development|PrintString (Utilities|String|ToString(Integer) _output_get)))

(fn ConstructionScript
  (|CallParentFunction))