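; BP_SKGun is the hero character's gun, providing automatic projectile fire while its trigger is active.
; BeginPlay caches a reference to the player's BP_HaroChar.
; ActiveTrigger fires at once, then starts a looping timer paced by ShootPerSecond, which DeactiveTrigger clears.
; Each Fire call spawns a BP_Projectil at the location and rotation of the character's ArrowProjectil component rather than from the gun itself.
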(event Custom|ActiveTrigger
  ;[1 1 1] Fire/Trigger
  (CallFunction|Fire)
  (Utilities|Time|SetTimerbyFunctionName 0 "Fire" (/ 1.0 (Variables|Default|GetShootPerSecond)) true))

(event Custom|DeactiveTrigger
  ;[1 1 1] Fire/Trigger
  (Utilities|Time|ClearTimerbyFunctionName 0 "Fire"))

(event EventBeginPlay
  ;[1 1 1] Get HeroChar Refer
  (bind _asbp_haro_char (Utilities|Casting|CastToBP_HaroChar (Game|GetPlayerCharacter 0)))
  (Variables|Default|SetHaroRefer _asbp_haro_char))

(fn ConstructionScript)

(fn Fire
  (bind _harorefer (Variables|Default|GetHaroRefer))
  (bind _arrowprojectil (Variables|/Game/HeroChar/BP_HaroChar.BP_HaroChar_C|GetArrowProjectil _harorefer))
  (bind _returnvalue (Transformation|GetWorldTransform _arrowprojectil))
  (Game|SpawnActorfromClass "/Game/HeroChar/Gun/BP_Projectil.BP_Projectil_C" (Math|Transform|MakeTransform (.location _returnvalue) (.rotation _returnvalue) "1,1,1") "Undefined" 0 0))